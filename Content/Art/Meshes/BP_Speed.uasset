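; BP_Speed is an engine order lever whose handle tilts to show the current speed.
; UpdateHandlePos scales MaxRot by the ratio of current speed to the range maximum to get a target pitch, then restarts the Alpha timeline.
; Each timeline update lerps from the handle's live relative rotation toward that target along the shortest path, so the motion compounds rather than following the raw curve.
; The construction script's instant-rotation logic is unconnected.
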(event Custom|UpdateHandlePos
  (params (MinMax :type Vector%202D%20Structure) (CurrSpeed :type Float%20%28single-precision%29))
  (Variables|Default|SetTargetRot (* (Variables|Default|GetMaxRot) (/ CurrSpeed (.Y (Math|Vector2D|BreakVector2D MinMax)))))
  (bind _newtrack_0 (Timeline|Alpha PlayFromStart)
    (:Update
      (Transformation|SetRelativeRotation (Variables|Default|GetEngineOrderHandle) (Math|Rotator|MakeRotator (.roll (Math|Rotator|Lerp(Rotator) (Variables|/Script/Engine.SceneComponent|GetRelativeRotation (Variables|Default|GetEngineOrderHandle)) (Math|Rotator|MakeRotator 0.0 (Variables|Default|GetTargetRot) 0.0) _newtrack_0 true)) (.pitch (Math|Rotator|Lerp(Rotator) (Variables|/Script/Engine.SceneComponent|GetRelativeRotation (Variables|Default|GetEngineOrderHandle)) (Math|Rotator|MakeRotator 0.0 (Variables|Default|GetTargetRot) 0.0) _newtrack_0 true)) (.yaw (Math|Rotator|Lerp(Rotator) (Variables|/Script/Engine.SceneComponent|GetRelativeRotation (Variables|Default|GetEngineOrderHandle)) (Math|Rotator|MakeRotator 0.0 (Variables|Default|GetTargetRot) 0.0) _newtrack_0 true))) false false))))

(event Collision|EventActorBeginOverlap
  (params (OtherActor :type Actor%20Object%20Reference)))

(fn ConstructionScript)