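; BP_Wave is a moving wave actor that flags floating objects while they overlap its mesh.
; Each Tick it shifts a fixed step along negative world X without sweeping, so its speed depends on frame rate.
; Begin and end overlap events on the StaticMesh set or clear IsInAWave on every Float_Comp component of the other actor.
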(event OnComponentBeginOverlap(StaticMesh)
  (params (OverlappedComponent :type Primitive%20Component%20Object%20Reference) (OtherActor :type Actor%20Object%20Reference) (OtherComp :type Primitive%20Component%20Object%20Reference) (OtherBodyIndex :type Integer) (bFromSweep :type Boolean) (SweepResult :type Hit%20Result%20Structure%20%28by%20ref%29))
  (for _array_element (Actor|GetComponentsByClass OtherActor "/Game/Waves/Float_Comp.Float_Comp_C")
    (Variables|/Game/Waves/Float_Comp.Float_Comp_C|SetbIsInAWave _array_element true)))

(event OnComponentEndOverlap(StaticMesh)
  (params (OverlappedComponent :type Primitive%20Component%20Object%20Reference) (OtherActor :type Actor%20Object%20Reference) (OtherComp :type Primitive%20Component%20Object%20Reference) (OtherBodyIndex :type Integer))
  (for _array_element (Actor|GetComponentsByClass OtherActor "/Game/Waves/Float_Comp.Float_Comp_C")
    (Variables|/Game/Waves/Float_Comp.Float_Comp_C|SetbIsInAWave _array_element false)))

(event Collision|EventActorBeginOverlap
  (params (OtherActor :type Actor%20Object%20Reference)))

(event EventTick
  (params (DeltaSeconds :type Float%20%28single-precision%29))
  (Transformation|SetActorLocation (+ (Transformation|GetActorLocation) "-30.000000,0.000000, 0") false false))

(fn ConstructionScript)